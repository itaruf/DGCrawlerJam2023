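; Blueprint function library of stat helpers for character XP progression and stat growth.
; SetCurrentXPProgression fires the level-up call on the stats component when XP reaches the requirement, then recurses with the leftover on the current level's data row.
; A requirement of -1 marks max level and zeroes XP.
; Separate formulas raise HP, ATK and DEF by random ranges and Energy by a fixed step; SetStatValue is an empty stub.
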(fn SetStatValue)

(fn SetCurrentXPProgression
  (params (Stats :type S%20Stats%20Structure) (New%20XP%20Value :type Float%20%28double-precision%29) (Current%20XP%20Value :type Float%20%28double-precision%29) (AC%20Stats :type AC%20Player%20Stats%20Object%20Reference))
  ;[1 1 1] Level Max ?
  (if (!= (.xprequired Stats) -1.0)
    (LocalVariables|SetL%20New%20XP%20Value New%20XP%20Value)
    (LocalVariables|SetL%20XP%20Required (.xprequired Stats))
    (LocalVariables|SetL%20Current%20XP%20Value Current%20XP%20Value)
    (if (or (>= (LocalVariables|GetL%20New%20XP%20Value) (LocalVariables|GetL%20XP%20Required)) (>= (+ (LocalVariables|GetL%20New%20XP%20Value) (LocalVariables|GetL%20Current%20XP%20Value)) (LocalVariables|GetL%20XP%20Required)))
      (Development|PrintString 0 "TRUE")
      (LocalVariables|SetL%20New%20XP%20Value (- (LocalVariables|GetL%20New%20XP%20Value) (- (LocalVariables|GetL%20XP%20Required) (LocalVariables|GetL%20Current%20XP%20Value))))
      (LocalVariables|SetL%20Current%20XP%20Value 0.0)
      ;[1 1 1] Update Data Stats
      (Default|CallEDIonLevelUP AC%20Stats (Utilities|Struct|MakeS_Stats (.level Stats) (.xprequired Stats) (.hp Stats) (.energy Stats) (.atk Stats) (.def Stats) (.cc Stats)))
      (CallFunction|SetCurrentXPProgression (Utilities|Array|Get(acopy) (Variables|/Game/DGCrawlerJam2023/Blueprints/Components/AC_PlayerStats.AC_PlayerStats_C|GetData%20Stats%20 AC%20Stats) (- (Variables|/Game/DGCrawlerJam2023/Blueprints/Components/AC_PlayerStats.AC_PlayerStats_C|GetCurrent%20Level AC%20Stats) 1)) (LocalVariables|GetL%20New%20XP%20Value) (LocalVariables|GetL%20Current%20XP%20Value) AC%20Stats)
      (else
        ;[1 1 1] No Level UP
        (Variables|/Game/DGCrawlerJam2023/Blueprints/Components/AC_PlayerStats.AC_PlayerStats_C|SetCurrent%20XP AC%20Stats (+ (LocalVariables|GetL%20New%20XP%20Value) (LocalVariables|GetL%20Current%20XP%20Value)))))
    (else
      (Variables|/Game/DGCrawlerJam2023/Blueprints/Components/AC_PlayerStats.AC_PlayerStats_C|SetCurrent%20XP AC%20Stats 0.0))))

(fn GetNewATKwithFormula
  (params (Current%20ATK :type Float%20%28double-precision%29))
  (return (+ Current%20ATK (Math|Random|RandomFloatinRange 4.0 6.0))))

(fn GetNewDefwithFormula
  (params (Current%20Def :type Float%20%28double-precision%29))
  (return (+ Current%20Def (Math|Random|RandomFloatinRange 2.0 4.0))))

(fn GetNewEnergywithFormula
  (params (Current%20Energy :type Float%20%28double-precision%29))
  (return (+ Current%20Energy 5.0)))

(fn GetNewHPwithFormula
  (params (Current%20HP :type Float%20%28double-precision%29))
  (return (+ Current%20HP (Math|Random|RandomFloatinRange 8.0 1e+01))))