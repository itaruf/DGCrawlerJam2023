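; BPFL_PropsHelper is a helper function library for props with a single direction-to-vector function.
; GetNormalVectorByDirection takes an actor and a six-way direction value and returns the matching axis vector in that actor's orientation.
; Forward, Right and Up come straight from the actor's direction vectors, while Backward, Left and Down negate them.
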(fn GetNormalVectorbyDirection
  (params (m_Actor :type Actor%20Object%20Reference) (Direction :type E_Direction%20Enum :default "NewEnumerator0"))
  (LocalVariables|SetActor m_Actor)
  (switch Utilities|FlowControl|Switch|SwitchonE_Direction Direction
    (:NewEnumerator0
      (return (Transformation|GetActorForwardVector (LocalVariables|GetActor))))
    (:NewEnumerator1
      (return (* (Transformation|GetActorForwardVector (LocalVariables|GetActor)) -1)))
    (:NewEnumerator2
      (return (* (Transformation|GetActorRightVector (LocalVariables|GetActor)) -1)))
    (:NewEnumerator3
      (return (Transformation|GetActorRightVector (LocalVariables|GetActor))))
    (:NewEnumerator4
      (return (Transformation|GetActorUpVector (LocalVariables|GetActor))))
    (:NewEnumerator5
      (return (* (Transformation|GetActorUpVector (LocalVariables|GetActor)) -1)))))