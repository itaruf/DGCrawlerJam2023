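; Blueprint function library that gives access to the grid cells and cell occupancy stored in BP_GameState for a dungeon crawler.
; Occupancy lives in two mirrored maps, actor-to-cell and cell-to-actor, with actor lookups falling back to GetCurrentOccupiedCellByLTBC when unmapped.
; SetCellOccupant writes both maps, updates the cell's occupied state and prints a debug string.
; An invalid occupant clears only the cell-side entry and marks the cell unoccupied.
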(fn GetAllCells
  (return (Variables|/Game/DGCrawlerJam2023/Blueprints/GameStates/BP_GameState.BP_GameState_C|GetCells (CallFunction|GetGameState))))

(fn GetGameState
  (bind _asbp_game_state (Utilities|Casting|CastToBP_GameState (Game|GetGameState))
    (:then
      (return _asbp_game_state))
    (:CastFailed
      (return 0))))

(fn GetCellOccupiedfromActor
  (params (Actor :type Actor%20Object%20Reference))
  (bind _game_state (CallFunction|GetGameState))
  (bind _actoroccupantandassociatedcell (Variables|/Game/DGCrawlerJam2023/Blueprints/GameStates/BP_GameState.BP_GameState_C|GetActorOccupantAndAssociatedCell _game_state))
  (bind (_value _returnvalue) (Utilities|Map|Find _actoroccupantandassociatedcell Actor))
  (if _returnvalue
    (return _value)
    (else
      (return (CallFunction|GetCurrentOccupiedCellbyLTBC "NewEnumerator5" Actor)))))

(fn GetActorfromOccupiedCell
  (params (Cell :type BP%20Cell%20Object%20Reference))
  (bind _game_state (CallFunction|GetGameState))
  (bind _cellandassociatedoccupant (Variables|/Game/DGCrawlerJam2023/Blueprints/GameStates/BP_GameState.BP_GameState_C|GetCellAndAssociatedOccupant _game_state))
  (bind (_value _returnvalue) (Utilities|Map|Find _cellandassociatedoccupant Cell))
  (if _returnvalue
    (return _value)
    (else
      (return 0))))

(fn SetCellOccupant
  (params (Selected%20Cell :type BP%20Cell%20Object%20Reference) (New%20Occupant :type Actor%20Object%20Reference))
  (bind _game_state (CallFunction|GetGameState))
  (bind _cellandassociatedoccupant (Variables|/Game/DGCrawlerJam2023/Blueprints/GameStates/BP_GameState.BP_GameState_C|GetCellAndAssociatedOccupant _game_state))
  (LocalVariables|SetSelectedCell Selected%20Cell)
  (bind _output_get (LocalVariables|SetNewOccupant New%20Occupant))
  (Utilities|IsValid _output_get
    (:Is%20Valid
      (Utilities|Map|Add (Variables|/Game/DGCrawlerJam2023/Blueprints/GameStates/BP_GameState.BP_GameState_C|GetActorOccupantAndAssociatedCell _game_state) (LocalVariables|GetNewOccupant) (LocalVariables|GetSelectedCell))
      (Utilities|Map|Add _cellandassociatedoccupant (LocalVariables|GetSelectedCell) (LocalVariables|GetNewOccupant))
      (Utilities|IsValid (LocalVariables|GetSelectedCell)
        (:Is%20Valid
          (CallFunction|SetCellOccupiedState true (LocalVariables|GetSelectedCell)))
        (:Is%20Not%20Valid
          (CallFunction|SetCellOccupiedState false (LocalVariables|GetSelectedCell) :!label _label))))
    (:Is%20Not%20Valid
      (Utilities|Map|Add _cellandassociatedoccupant (LocalVariables|GetSelectedCell) (LocalVariables|GetNewOccupant))
      (goto _label)))
  (Development|PrintString 0 (Utilities|String|Append "OWNER : " (Utilities|GetDisplayName (LocalVariables|GetNewOccupant)) (Utilities|String|Append "- CELL : " (Utilities|GetDisplayName (LocalVariables|GetSelectedCell))))))

(fn GetCellOccupantsMap
  (return (Variables|/Game/DGCrawlerJam2023/Blueprints/GameStates/BP_GameState.BP_GameState_C|GetActorOccupantAndAssociatedCell (CallFunction|GetGameState))))

(fn GetCellMap
  (return (Variables|/Game/DGCrawlerJam2023/Blueprints/GameStates/BP_GameState.BP_GameState_C|GetCellAndAssociatedOccupant (CallFunction|GetGameState (LocalVariables|Get__WorldContext)))))