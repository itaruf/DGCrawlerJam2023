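; Blueprint function library of static helpers for reaching and manipulating the player from other Blueprints.
; GetPlayer casts player pawn 0 to BP_Player and underpins getters for controller, position, rotation and six-way direction vectors.
; Setters set location without sweep, set rotation, or yaw the capsule by TurnDegree, leaving the AxisValue product unused.
; SetPlayerPositionWithUnit is unfinished: its direction switch moves nothing.
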(fn GetPlayer
  (bind _asbp_player (Utilities|Casting|CastToBP_Player (Game|Player|GetPlayerPawn 0))
    (:then
      (return _asbp_player))
    (:CastFailed
      (Development|PrintString 0 "FAILED"))))

(fn GetPlayerRotation
  (return (Transformation|GetActorRotation (CallFunction|GetPlayer))))

(fn GetPlayerPosition
  (return (Transformation|GetActorLocation (CallFunction|GetPlayer (LocalVariables|Get__WorldContext)))))

(fn GetPlayerNormalVectorbyDirection
  (params (Direction :type E_Direction%20Enum :default "NewEnumerator0"))
  (LocalVariables|SetPlayer (CallFunction|GetPlayer (LocalVariables|Get__WorldContext)))
  (switch Utilities|FlowControl|Switch|SwitchonE_Direction Direction
    (:NewEnumerator0
      (return (Transformation|GetActorForwardVector (LocalVariables|GetPlayer))))
    (:NewEnumerator1
      (return (* (Transformation|GetActorForwardVector (LocalVariables|GetPlayer)) -1)))
    (:NewEnumerator2
      (return (* (Transformation|GetActorRightVector (LocalVariables|GetPlayer)) -1)))
    (:NewEnumerator3
      (return (Transformation|GetActorRightVector (LocalVariables|GetPlayer))))
    (:NewEnumerator4
      (return (Transformation|GetActorUpVector (LocalVariables|GetPlayer))))
    (:NewEnumerator5
      (return (* (Transformation|GetActorUpVector (LocalVariables|GetPlayer)) -1)))))

(fn GetPlayerController
  (bind _asbp_player_controller (Utilities|Casting|CastToBP_PlayerController (Pawn|GetController (CallFunction|GetPlayer (LocalVariables|Get__WorldContext)))))
  (return _asbp_player_controller))

(fn SetPlayerPosition
  (params (New%20Position :type Vector))
  (Transformation|SetActorLocation (CallFunction|GetPlayer) New%20Position false false))

(fn SetPlayerPositionwithUnit
  (params (Unit%20To%20Travel :type Float%20%28double-precision%29) (Direction :type E_Direction%20Enum :default "NewEnumerator0"))
  (LocalVariables|SetUnitToTravel Unit%20To%20Travel)
  (switch Utilities|FlowControl|Switch|SwitchonE_Direction Direction))

(fn SetPlayerRotationwithInput
  (params (Axis%20Value :type Float%20%28double-precision%29))
  (bind _player_rotation (CallFunction|GetPlayerRotation))
  (LocalVariables|SetTurn%20Degree (LocalVariables|GetTurn%20Degree))
  (Transformation|SetWorldRotation (Variables|/Script/Engine.Character|GetCapsuleComponent (CallFunction|GetPlayer)) (Math|Rotator|MakeRotator (.roll _player_rotation) (.pitch _player_rotation) (+ (.yaw _player_rotation) (LocalVariables|GetTurn%20Degree))) false false))

(fn SetPlayerRotation
  (params (New%20Rotation :type Rotator))
  (Transformation|SetActorRotation (CallFunction|GetPlayer) New%20Rotation))