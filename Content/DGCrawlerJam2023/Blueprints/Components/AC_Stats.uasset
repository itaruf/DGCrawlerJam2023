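; Actor component that holds its owner's level, XP requirement, HP, energy and combat stats, with event bindings for game start and level-up.
; SetStats loads rows from a stats DataTable and initializes current values from the first.
; SetStatFromLevel takes the next row's level, XP requirement and CC, deriving other stats through formulas.
; C key adds XP, apparently for debugging; SetHP and SetEnergy are empty stubs.
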(event Custom|Set%20Stats
  (bind _data_stats_ (Variables|Default|GetData%20Stats%20))
  (bind _data_stats__2 (Variables|Default|GetData%20Stats%20))
  (bind _output (Utilities|Array|Get(acopy) _data_stats__2))
  (bind (_level _xprequired _hp _energy _atk _def _cc) (Utilities|Struct|BreakS_Stats _output))
  (bind _outrownames (DataTable|GetDataTableRowNames (Variables|Default|GetData%20Table%20Stats)))
  (for _array_element _outrownames
    (bind _returnvalue (Utilities|GetDataTableRow (Variables|Default|GetData%20Table%20Stats) _array_element)
      (:then
        (Utilities|Array|AddUnique (Variables|Default|GetData%20Stats%20) _returnvalue))))
  (Variables|CurrentStats|SetCurrent%20Level _level)
  (Variables|CurrentStats|SetCurrent%20HP _hp)
  (Variables|CurrentStats|SetCurrent%20Energy _energy)
  (Variables|CurrentStats|SetCurrent%20ATK _atk)
  (Variables|CurrentStats|SetCurrent%20DEF _def)
  (Variables|CurrentStats|SetCurrent%20CC%20%25 _cc)
  (if (> (Utilities|Array|Length _data_stats_) 1)
    (Variables|CurrentStats|SetCurrent%20XP%20Required (Utilities|Struct|BreakS_Stats (Utilities|Array|Get(acopy) _data_stats_ 1)))
    (else
      (Variables|CurrentStats|SetCurrent%20XP%20Required _xprequired))))

(event Custom|Set%20Stat%20From%20Level
  (params (Current%20Stat :type S%20Stats%20Structure))
  (bind _level (Utilities|Struct|BreakS_Stats Current%20Stat))
  (bind (_hp _energy _atk _def) (Utilities|Struct|BreakS_Stats Current%20Stat))
  (bind _data_stats_ (Variables|Default|GetData%20Stats%20))
  (bind _returnvalue (+ _level 1))
  (bind _returnvalue_2 (- _returnvalue 1))
  (bind _output (Utilities|Array|Get(acopy) _data_stats_ _returnvalue_2))
  (bind (_level_2 _xprequired _cc) (Utilities|Struct|BreakS_Stats _output))
  (if (<= _returnvalue (Utilities|Array|Length (Variables|Default|GetData%20Stats%20)))
    (Variables|CurrentStats|SetCurrent%20Level _level_2)
    (Variables|CurrentStats|SetCurrent%20XP%20Required _xprequired)
    (bind _output_get (Variables|CurrentStats|SetCurrent%20HP (CallFunction|GetNewHPwithFormula _hp)))
    (Variables|CurrentStats|SetCurrent%20Energy (CallFunction|GetNewEnergywithFormula _energy))
    (Variables|CurrentStats|SetCurrent%20ATK (CallFunction|GetNewATKwithFormula _atk))
    (Variables|CurrentStats|SetCurrent%20DEF (CallFunction|GetNewDefwithFormula _def))
    (Variables|CurrentStats|SetCurrent%20CC%20%25 _cc)
    (Development|PrintString (Utilities|String|ToString(Float) _output_get))))

(event EventBeginPlay
  (bind _returnvalue (Components|GetOwner))
  (Utilities|FlowControl|Sequence
    (:then_0
      (EventDispatchers|BindEventtoEDIStartGame (CallFunction|GetGameMode) (EventDispatchers|CreateEvent :!event Custom|Set%20Stats))
      (EventDispatchers|BindEventtoEDIonLevelUP (EventDispatchers|CreateEvent :!event Custom|Set%20Stat%20From%20Level)))
    (:then_1
      (Variables|Default|SetOwner _returnvalue)
      (Input|EnableInput _returnvalue (CallFunction|GetPlayerController)))))

(event EventTick
  (params (DeltaSeconds :type Float%20%28single-precision%29)))

(event Input|KeyboardEvents|V
  (params (Key :type Key%20Structure :default "None")))

(event Input|KeyboardEvents|C
  (params (Key :type Key%20Structure :default "None"))
  (bind _self self)
  (:Pressed
    (CallFunction|SetCurrentXPProgression (Utilities|Struct|MakeS_Stats (Variables|CurrentStats|GetCurrent%20Level) (Variables|CurrentStats|GetCurrent%20XP%20Required) (Variables|CurrentStats|GetCurrent%20HP) (Variables|CurrentStats|GetCurrent%20Energy) (Variables|CurrentStats|GetCurrent%20ATK) (Variables|CurrentStats|GetCurrent%20DEF) (Variables|CurrentStats|GetCurrent%20CC%20%25)) 15.0 (Variables|CurrentStats|GetCurrent%20XP _self) _self)))

(fn SetHP)

(fn SetEnergy)