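; Sanity actor component that tracks an integer sanity value and can drain it over time.
; BeginPlay binds to the game mode's start-game dispatcher, and start/end events control a looping drain timer.
; The drain only runs while sanity is strictly between min and max, so a value at either limit stays put.
; Each drain clamps the value, picks one of two states by whether it is below zero, and broadcasts value and state.
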(event Custom|Event%20Loose%20Sanity%20Over%20Time
  (if (not (or (<= (Variables|Default|GetCurrent%20Sanity) (Variables|Default|GetMin%20Sanity)) (>= (Variables|Default|GetCurrent%20Sanity) (Variables|Default|GetMax%20Sanity))))
    (bind _output_get (Variables|Default|SetCurrent%20Sanity (Math|Integer|Clamp(Integer) (- (Variables|Default|GetCurrent%20Sanity) (Variables|Default|GetSanity%20Loss%20Over%20Time)) (Variables|Default|GetMin%20Sanity) (Variables|Default|GetMax%20Sanity))))
    (Default|CallEDIonSanityUpdated _output_get)
    (if (< _output_get 0)
      (CallFunction|SetCurrentSanityState self "NewEnumerator1")
      (else
        (CallFunction|SetCurrentSanityState self "NewEnumerator0")))
    (Default|CallEDIonSanityStateChanged self (Variables|Default|GetCurrent%20Sanity%20State))))

(event Custom|Event%20Start%20Loose%20Sanity%20Over%20Time
  (bind _returnvalue (Utilities|Time|SetTimerbyEvent (EventDispatchers|CreateEvent :!event Custom|Event%20Loose%20Sanity%20Over%20Time) (Variables|Default|GetSanity%20Loss%20Timer%20In%20Seconds) true))
  (Variables|Default|SetLoose%20Sanity%20Over%20Time%20Timer _returnvalue))

(event Custom|Event%20End%20Loose%20Sanity%20Over%20Time
  (Utilities|Time|ClearandInvalidateTimerbyHandle (Variables|Default|GetLoose%20Sanity%20Over%20Time%20Timer)))

(event EventBeginPlay
  (EventDispatchers|BindEventtoEDIStartGame (CallFunction|GetGameMode) (EventDispatchers|CreateEvent :!event Custom|Event%20Start%20Loose%20Sanity%20Over%20Time)))