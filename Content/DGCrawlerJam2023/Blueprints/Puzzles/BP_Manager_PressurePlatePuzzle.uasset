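; Manager for a pressure plate puzzle where symbols must be activated in a set order.
; It binds to overlap events on the plates in a plate-to-symbol map, and each press toggles that symbol and updates the current order list.
; When an added symbol makes that list match the solution's length, the orders are compared.
; Success unbinds the plates, while failure deactivates all symbols and clears the list.
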(event Custom|On%20Pressure%20Plate%20Overlapped
  (params (Pressure%20Overlapped :type BP%20Pressure%20Plate%20Object%20Reference))
  (bind _pressure_plates (Variables|PressurePlates&AssociatedSymbol|GetPressure%20Plates))
  (bind (_value _returnvalue) (Utilities|Map|Find _pressure_plates Pressure%20Overlapped))
  (Utilities|IsValid _value
    (:Is%20Valid
      (if _returnvalue
        (Variables|PressurePlate|SetPressure%20Plate Pressure%20Overlapped)
        (bind _output_get (Variables|Symboles|SetAssociated%20Symbole _value))
        (if (Variables|/Game/DGCrawlerJam2023/Blueprints/Puzzles/BP_Symbol.BP_Symbol_C|GetIs%20Activated _output_get)
          (Default|OnDeactivation (Variables|Symboles|GetAssociated%20Symbole))
          (Utilities|Array|RemoveItem (Variables|Symboles|GetCurrent%20Symbol%20Order) (Variables|Symboles|GetAssociated%20Symbole))
          (else
            (Default|OnActivation (Variables|Symboles|GetAssociated%20Symbole))
            (Utilities|Array|Add (Variables|Symboles|GetCurrent%20Symbol%20Order) (Variables|Symboles|GetAssociated%20Symbole))
            (CallFunction|OnPuzzleProgressing)))))))

(event EventBeginPlay
  (Utilities|FlowControl|Sequence
    (:then_0
      _)
    (:then_1
      _))
  (bind _keys (Utilities|Map|Keys (Variables|PressurePlates&AssociatedSymbol|GetPressure%20Plates)))
  (for _array_element _keys
    (EventDispatchers|BindEventtoEDIonPlayerBeginOverlapPressure _array_element (EventDispatchers|CreateEvent :!event Custom|On%20Pressure%20Plate%20Overlapped))))

(event Collision|EventActorBeginOverlap
  (params (OtherActor :type Actor%20Object%20Reference)))

(event EventTick
  (params (DeltaSeconds :type Float%20%28single-precision%29)))

(event EventOnPuzzleProgressing
  (if (== (Utilities|Array|Length (Variables|SuccessCondition|GetSymbol%20Order%20To%20Success%20)) (Utilities|Array|Length (Variables|Symboles|GetCurrent%20Symbol%20Order)))
    (Variables|Default|SetSuccess true)
    (bind (_array_element _array_index) (Utilities|Array|ForEachLoopwithBreak (Variables|SuccessCondition|GetSymbol%20Order%20To%20Success%20) :!label _label)
      (:LoopBody
        (if (not (== _array_element (Utilities|Array|Get(acopy) (Variables|Symboles|GetCurrent%20Symbol%20Order) _array_index)))
          (Variables|Default|SetSuccess false)
          (goto _label Break)))
      (:Completed
        (if (Variables|Default|GetSuccess)
          (CallFunction|OnPuzzleSolved)
          (else
            (CallFunction|OnPuzzleFailed)))))))

(event EventOnPuzzleSolved
  (bind _keys (Utilities|Map|Keys (Variables|PressurePlates&AssociatedSymbol|GetPressure%20Plates)))
  (for _array_element _keys
    (EventDispatchers|UnbindEventfromEDIonPlayerBeginOverlapPressure _array_element (EventDispatchers|CreateEvent :!event Custom|On%20Pressure%20Plate%20Overlapped))))

(event EventOnPuzzleFailed
  (Development|PrintString "FAILED")
  (bind _values (Utilities|Map|Values (Variables|PressurePlates&AssociatedSymbol|GetPressure%20Plates)))
  (for _array_element _values
    (Class|BPIStatus|OnDeactivation(Message) _array_element))
  (Utilities|Array|Clear (Variables|Symboles|GetCurrent%20Symbol%20Order)))

(fn ConstructionScript
  (|CallParentFunction))