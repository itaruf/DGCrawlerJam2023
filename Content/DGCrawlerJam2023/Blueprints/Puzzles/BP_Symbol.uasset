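; BP_Symbol is a puzzle symbol actor that shows whether it is activated by lighting up.
; Its point light is switched off and hidden on BeginPlay.
; OnActivation and OnDeactivation events toggle the light's active state and visibility and record the result in IsActivated, with no trigger logic of its own.
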(event EventBeginPlay
  (Components|Activation|Deactivate (Variables|Default|GetPointLight))
  (Rendering|SetVisibility (Variables|Default|GetPointLight) false false))

(event Collision|EventActorBeginOverlap
  (params (OtherActor :type Actor%20Object%20Reference)))

(event EventTick
  (params (DeltaSeconds :type Float%20%28single-precision%29)))

(event EventOnDeactivation
  (Components|Activation|Deactivate (Variables|Default|GetPointLight))
  (Rendering|SetVisibility (Variables|Default|GetPointLight) false false)
  (Variables|Default|SetIs%20Activated false))

(event EventOnActivation
  (Components|Activation|Activate (Variables|Default|GetPointLight) false)
  (Rendering|SetVisibility (Variables|Default|GetPointLight) true false)
  (Variables|Default|SetIs%20Activated true))

(fn ConstructionScript)