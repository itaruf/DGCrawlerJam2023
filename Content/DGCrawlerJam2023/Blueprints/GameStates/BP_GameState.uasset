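; Game state for the grid crawler that keeps a registry of the cells in the level and their occupants.
; On BeginPlay it collects every BP_Cell actor and adds each as a key to CellAndAssociatedOccupant with no occupant assigned.
; OnFindOccupiedCell forwards a player interact message to the occupant.
; OnLeavePreviousCell is an empty stub, and the delegate binding node for occupied cells is left unconnected.
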(event Custom|Get%20All%20Cells
  (Utilities|FlowControl|Sequence
    (:then_0
      (bind _outactors (Actor|GetAllActorsOfClass "/Game/DGCrawlerJam2023/Blueprints/Art/Blueprints/Environments/Cells/BP_Cell.BP_Cell_C"))
      (Variables|Cell|SetCells _outactors))
    (:then_1
      (for _array_element (Variables|Cell|GetCells)
        (Utilities|Map|Add (Variables|Cell|GetCellAndAssociatedOccupant) _array_element 0)))))

(event Custom|On%20Leave%20Previous%20Cell
  (params (Current%20Cell :type BP%20Cell%20Object%20Reference)))

(event Custom|On%20Find%20Occupied%20Cell
  (params (Actor%20Occupant :type Actor%20Object%20Reference))
  (Class|BPInteractionswithPlayer|OnPlayerInteractwith(Message) Actor%20Occupant))

(event EventBeginPlay
  (Utilities|FlowControl|Sequence
    (:then_0
      (CallFunction|GetAllCells))))

(fn ConstructionScript)