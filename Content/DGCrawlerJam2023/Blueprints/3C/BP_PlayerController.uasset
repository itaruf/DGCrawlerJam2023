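; Player controller for a grid-based dungeon crawler, handling stepped movement, turning, pause and the player info/inventory screen.
; Forward/backward input runs an obstacle trace, then either moves the player and updates cell occupancy or reports an occupied cell to the GameState.
; Per-direction flags gate input, with a short timer as an input buffer.
; It binds to GameState battle events and has helpers to toggle movement and save the pre-fight transform.
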(event Custom|OnBufferActivated
  (if (not (Utilities|Time|IsTimerActivebyHandle (Variables|Default|GetBufferTimer)))
    (CallFunction|SetPlayerMovementsState false)
    (bind _returnvalue (Utilities|Time|SetTimerbyEvent (EventDispatchers|CreateEvent :!event Custom|OnBufferDisabled) 0.05))
    (Variables|Default|SetBufferTimer _returnvalue)))

(event Custom|OnBufferDisabled
  (CallFunction|SetPlayerMovementsState true)
  (Utilities|Time|ClearandInvalidateTimerbyHandle (Variables|Default|GetBufferTimer)))

(event EventBeginPlay
  (Utilities|FlowControl|Sequence
    (:then_0
      (Input|EnableInput (CallFunction|GetPlayer) (CallFunction|GetPlayerController))
      (EventDispatchers|BindEventtoEDIonMove (EventDispatchers|CreateEvent :!event Custom|OnBufferActivated)))
    (:then_1
      (EventDispatchers|BindEventtoEDIStartBattle (CallFunction|GetGameState) (EventDispatchers|CreateEvent :!event DisableMovement))
      (EventDispatchers|BindEventtoEDIBeforeStartBattle (CallFunction|GetGameState) (EventDispatchers|CreateEvent :!event SavePlayerTransform))
      (EventDispatchers|BindEventtoEDIBeforeStartBattle (CallFunction|GetGameState) (EventDispatchers|CreateEvent :!event DisableMovement)))
    (:then_2
      (EventDispatchers|BindEventtoEDIEndBattle (CallFunction|GetGameState) (EventDispatchers|CreateEvent :!event EnableMovement)))))

(event EventTick
  (params (DeltaSeconds :type Float%20%28single-precision%29)))

(event Input|ActionEvents|InputActionMoveRight
  (params (Key :type Key%20Structure :default "None"))
  (:Pressed
    (if (Variables|Default|GetCan%20Player%20Move%20Right)
      (Default|CallEDIonMove)
      (CallFunction|SetPlayerRotationwithInput 1.0)
      (Default|CallEDIonTurn))))

(event Input|ActionEvents|InputActionMoveLeft
  (params (Key :type Key%20Structure :default "None"))
  (:Pressed
    (if (Variables|Default|GetCan%20Player%20Move%20Left)
      (Default|CallEDIonMove)
      (CallFunction|SetPlayerRotationwithInput -1.0)
      (Default|CallEDIonTurn))))

(event Input|ActionEvents|InputActionMoveForward
  (params (Key :type Key%20Structure :default "None"))
  (:Pressed
    (if (Variables|Default|GetCan%20Player%20Move%20FW)
      (CallFunction|MoveFW/BW "NewEnumerator0"))))

(event Input|ActionEvents|InputActionMoveBackward
  (params (Key :type Key%20Structure :default "None"))
  (:Pressed
    (if (Variables|Default|GetCan%20Player%20Move%20BW)
      (CallFunction|MoveFW/BW "NewEnumerator1"))))

(event Input|ActionEvents|InputActionPause
  (params (Key :type Key%20Structure :default "None"))
  (:Pressed
    (Utilities|FlowControl|FlipFlop
      (:A
        (Game|SetGamePaused true))
      (:B
        (Game|SetGamePaused false)))
    (Default|CallEDITogglePause)))

(event Input|ActionEvents|InputActionPlayerInfo
  (params (Key :type Key%20Structure :default "None"))
  (:Pressed
    (if (not (Variables|/Game/DGCrawlerJam2023/Blueprints/GameStates/BP_GameState.BP_GameState_C|GetIsInFight (CallFunction|GetGameState)))
      (Utilities|FlowControl|FlipFlop
        (:A
          (Default|CallEDIonInventoryOpened (CallFunction|GetPlayerInventoryComponent))
          (Default|CallEDIonDisplayPlayerInfo)
          (CallFunction|SetPlayerMovementsState false))
        (:B
          (Default|CallEDIonInventoryClosed (CallFunction|GetPlayerInventoryComponent))
          (Default|CallEDIonClosePlayerInfo)
          (CallFunction|SetPlayerMovementsState true))))))

(fn ConstructionScript)

(fn SetPlayerMovementsState
  (params (New%20State :type Boolean))
  (bind _output_get (Variables|Default|SetCan%20Player%20Move%20FW New%20State))
  (bind _output_get_2 (Variables|Default|SetCan%20Player%20Move%20Right _output_get))
  (bind _output_get_3 (Variables|Default|SetCan%20Player%20Move%20BW _output_get_2))
  (Variables|Default|SetCan%20Player%20Move%20Left _output_get_3))

(fn MoveFW/BW
  (params (m_Direction :type E_Direction%20Enum :default "NewEnumerator0"))
  (LocalVariables|SetDirection m_Direction)
  (Default|CallEDIonMove)
  (bind _out_hit_blocking_hit (CallFunction|IsPlayerBlocked "TraceTypeQuery3" (.obstaclecheckdistance (Utilities|Struct|MakeS_MovementData 5e+01 4e+02)) (LocalVariables|GetDirection)))
  (if (not _out_hit_blocking_hit)
    (LocalVariables|SetTargeted%20Cell (CallFunction|GetPlayerNextCellbyLTBC (LocalVariables|GetDirection)))
    (Utilities|IsValid (LocalVariables|GetTargeted%20Cell)
      (:Is%20Valid
        (if (CallFunction|IsCellOccupied (LocalVariables|GetTargeted%20Cell))
          (Default|OnFindOccupiedCell (CallFunction|GetGameState) (CallFunction|GetActorfromOccupiedCell (LocalVariables|GetTargeted%20Cell)))
          (else
            (CallFunction|SetCellOccupant (CallFunction|GetCellOccupiedfromActor (CallFunction|GetPlayer)))
            (CallFunction|SetCellOccupant (LocalVariables|GetTargeted%20Cell) (CallFunction|GetPlayer))
            (CallFunction|SetPlayerPosition (Transformation|GetWorldLocation (Variables|/Game/DGCrawlerJam2023/Blueprints/Art/Blueprints/Environments/Cells/BP_Cell.BP_Cell_C|GetCellLocation (LocalVariables|GetTargeted%20Cell))))))))))

(fn EnableMovement
  (Variables|Default|SetCan%20Player%20Move%20FW true)
  (Variables|Default|SetCan%20Player%20Move%20Right true)
  (Variables|Default|SetCan%20Player%20Move%20BW true)
  (Variables|Default|SetCan%20Player%20Move%20Left true)
  (Utilities|Time|ClearandInvalidateTimerbyHandle (Variables|Default|GetBufferTimer)))

(fn DisableMovement
  (Variables|Default|SetCan%20Player%20Move%20FW false)
  (Variables|Default|SetCan%20Player%20Move%20Right false)
  (Variables|Default|SetCan%20Player%20Move%20BW false)
  (Variables|Default|SetCan%20Player%20Move%20Left false)
  (Utilities|Time|ClearandInvalidateTimerbyHandle (Variables|Default|GetBufferTimer)))

(fn SavePlayerTransform
  (Variables|Default|SetPlayer%20Transform%20Before%20Fight (CallFunction|GetPlayerTransform)))