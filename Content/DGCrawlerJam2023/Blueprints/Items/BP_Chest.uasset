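; BP_Chest is a lootable chest item that gives the player an item when interacted with.
; It binds to the game mode's start-game dispatcher on BeginPlay, and OnSpawn registers it as the occupant of its grid cell.
; On first interaction it generates the item in the player's inventory, sets a looted flag, then after a short delay logs a pickup message and destroys itself.
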(event Custom|On%20Spawn
  (CallFunction|SetCellOccupant (CallFunction|GetCurrentOccupiedCellbyLTBC "NewEnumerator5" self) self))

(event EventBeginPlay
  (EventDispatchers|BindEventtoEDIStartGame (CallFunction|GetGameMode) (EventDispatchers|CreateEvent :!event Custom|On%20Spawn)))

(event EventOnPlayerInteractwith
  (if (not (Variables|Default|GetLooted))
    (bind _item_generated (Default|GenerateItem (CallFunction|GetPlayerInventoryComponent) (Variables|Default|GetItem)))
    (Variables|Default|SetLooted true)
    (Utilities|FlowControl|Delay 1.0)
    (Default|LogMessage (CallFunction|GetGameState) (Utilities|Text|ToText(String) (Utilities|String|Append (Utilities|GetDisplayName _item_generated) " added to the inventory !")))
    (Actor|DestroyActor)))

(fn ConstructionScript)