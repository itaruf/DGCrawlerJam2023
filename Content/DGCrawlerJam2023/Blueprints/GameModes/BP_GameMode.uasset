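; Game mode for a grid-based dungeon crawler that sets up the player and hosts debug controls for game flow.
; On BeginPlay it caches the player, enables input, registers the player as occupant of their starting cell and binds to the start-game dispatcher.
; Keys fire start-game, escape-battle and end-battle dispatchers or stop the fast looping timer started on game start.
; A diagnostic event prints whether the player's cell is occupied.
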(event Custom|On%20Start%20Game
  (bind _returnvalue (Utilities|Time|SetTimerbyEvent (EventDispatchers|CreateEvent :!event Custom|Event%20Get%20Information) 0.01 true))
  (Variables|Default|SetStart%20Game%20Timer _returnvalue))

(event Custom|Event%20Get%20Information
  (bind _out_hit_blocking_hit (CallFunction|IsPlayerBlocked "TraceTypeQuery3" (.obstaclecheckdistance (Utilities|Struct|MakeS_MovementData 5e+01 2e+02)) "NewEnumerator0"))
  (Development|PrintString (Utilities|String|ToString(Boolean) (CallFunction|IsCellOccupied (CallFunction|GetCellOccupiedfromActor (CallFunction|GetPlayer))))))

(event Custom|On%20Stop%20Game
  (Utilities|Time|ClearandInvalidateTimerbyHandle (Variables|Default|GetStart%20Game%20Timer)))

(event EventBeginPlay
  (Utilities|FlowControl|Sequence
    (:then_0
      (CallFunction|InitializeData))
    (:then_1
      ;[1 1 1] Set Player Starting Cell
      (CallFunction|SetCellOccupant (CallFunction|GetCurrentOccupiedCellbyLTBC "NewEnumerator0" (CallFunction|GetPlayer)) (CallFunction|GetPlayer)))
    (:then_2
      (EventDispatchers|BindEventtoEDIStartGame (EventDispatchers|CreateEvent :!event Custom|On%20Start%20Game)))))

(event Input|KeyboardEvents|E
  (params (Key :type Key%20Structure :default "None"))
  (:Pressed
    (Default|CallEDIStartGame)))

(event Input|KeyboardEvents|R
  (params (Key :type Key%20Structure :default "None"))
  (:Pressed
    (CallFunction|OnStopGame)))

(event Input|KeyboardEvents|T
  (params (Key :type Key%20Structure :default "None"))
  (:Pressed
    (Default|CallEDIEscapeBattle)))

(event Input|KeyboardEvents|G
  (params (Key :type Key%20Structure :default "None"))
  (:Pressed
    (Default|CallEDIEndBattle)))

(fn ConstructionScript)

(fn InitializeData
  (Utilities|FlowControl|Sequence
    (:then_0
      (Variables|PlayerData|SetPlayer (CallFunction|GetPlayer)))
    (:then_1
      (Input|EnableInput (CallFunction|GetPlayerController)))))