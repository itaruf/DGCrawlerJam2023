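; Dungeon-crawler enemy spawner that starts a battle when the player walks into its collision and no fight is running.
; Its child-actor BP_EnemySymbol supplies the enemy class and is passed along with the spawner's overlap dispatcher.
; After firing the GameMode's start-battle dispatcher, it spawns that enemy at the fight manager's arena cell and registers it as the fight's enemy.
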(event OnComponentBeginOverlap(SpawnerCollision)
  (params (OverlappedComponent :type Primitive%20Component%20Object%20Reference) (OtherActor :type Actor%20Object%20Reference) (OtherComp :type Primitive%20Component%20Object%20Reference) (OtherBodyIndex :type Integer) (bFromSweep :type Boolean) (SweepResult :type Hit%20Result%20Structure%20%28by%20ref%29))
  (if (== OtherComp (CallFunction|GetPlayerCollisionComponent))
    (if (not (Variables|/Game/DGCrawlerJam2023/Blueprints/GameModes/BP_GameMode.BP_GameMode_C|GetIsInFight (CallFunction|GetGameMode)))
      (bind _asbp_enemy_symbol (Utilities|Casting|CastToBP_EnemySymbol (Variables|/Script/Engine.ChildActorComponent|GetChildActor (Variables|Default|GetEnemySpawned))))
      (Default|CallEDIonPlayerBeginOverlapSpawner _asbp_enemy_symbol)
      (Default|CallEDIStartBattle (CallFunction|GetGameMode))
      (CallFunction|SpawnEnemy))))

(event Custom|Spawn%20Enemy
  (bind _returnvalue (Game|SpawnActorfromClass (Variables|/Game/DGCrawlerJam2023/Blueprints/Spawners/BP_EnemySymbol.BP_EnemySymbol_C|GetEnemy%20Class (Variables|Default|GetEnemy%20Symbol)) (Math|Transform|MakeTransform (.location (Transformation|GetActorTransform (Variables|/Game/DGCrawlerJam2023/Blueprints/Fights/BP_Manager_Fight.BP_Manager_Fight_C|GetEnemy%20Cell%20Arena (Variables|/Game/DGCrawlerJam2023/Blueprints/GameModes/BP_GameMode.BP_GameMode_C|GetManager%20Fight (CallFunction|GetGameMode))))) "0, 0, 0" "1.000000,1.000000,1.000000") "AlwaysSpawn" 0 0))
  (Default|CallEDISetEnemyforFight (Variables|/Game/DGCrawlerJam2023/Blueprints/GameModes/BP_GameMode.BP_GameMode_C|GetManager%20Fight (CallFunction|GetGameMode)) _returnvalue))

(event EventBeginPlay
  (EventDispatchers|BindEventtoEDIStartBattle (CallFunction|GetGameMode) (EventDispatchers|CreateEvent :!event Custom|Spawn%20Enemy))
  (bind _asbp_enemy_symbol (Utilities|Casting|CastToBP_EnemySymbol (Variables|/Script/Engine.ChildActorComponent|GetChildActor (Variables|Default|GetEnemySpawned))))
  (Variables|Default|SetEnemy%20Symbol _asbp_enemy_symbol))

(event Collision|EventActorBeginOverlap
  (params (OtherActor :type Actor%20Object%20Reference)))

(event EventTick
  (params (DeltaSeconds :type Float%20%28single-precision%29)))

(fn ConstructionScript)