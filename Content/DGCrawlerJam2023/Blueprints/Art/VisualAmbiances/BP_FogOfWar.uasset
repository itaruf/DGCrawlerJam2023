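; Fog of war actor that keeps a height fog component on the player's position every tick.
; A rate-scaled timeline animates volumetric fog scattering distribution between min and max values, and each finish restarts it in reverse from the end a tick later.
; On BeginPlay it binds to the game mode's start-game dispatcher, and separate events start and stop the animation.
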(event Custom|Event%20Start%20Scattering%20Distribution
  (bind _value (Timeline|T%20Fog%20Scattering%20Distribution PlayFromStart)
    (:Update
      (Class|ExponentialHeightFogComponent|SetVolumetricFogScatteringDistribution (Variables|Default|GetHeightFogComponent) (Math|Float|Lerp (Variables|ScatteringDistribution|GetMin%20Scattering%20Distribution%20) (Variables|ScatteringDistribution|GetMax%20Scattering%20Distribution) _value)))
    (:Finished
      (Utilities|FlowControl|DelayUntilNextTick)
      (Timeline|T%20Fog%20Scattering%20Distribution ReverseFromEnd))))

(event Custom|Event%20Stop%20Scattering%20Distribution
  (Audio|Components|Audio|Stop (Variables|Default|GetT%20Fog%20Scattering%20Distribution)))

(event EventBeginPlay
  (EventDispatchers|BindEventtoEDIStartGame (CallFunction|GetGameMode) (EventDispatchers|CreateEvent :!event Custom|Event%20Start%20Scattering%20Distribution))
  (Components|Timeline|SetPlayRate (Variables|Default|GetT%20Fog%20Scattering%20Distribution) (Variables|ScatteringDistribution|GetScattering%20Distribution%20Speed%20Rate)))

(event Collision|EventActorBeginOverlap
  (params (OtherActor :type Actor%20Object%20Reference)))

(event EventTick
  (params (DeltaSeconds :type Float%20%28single-precision%29))
  (Transformation|SetWorldLocation (Variables|Default|GetHeightFogComponent) (CallFunction|GetPlayerPosition) false false))

(fn ConstructionScript)